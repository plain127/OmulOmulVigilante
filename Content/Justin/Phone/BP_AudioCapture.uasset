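; BP_AudioCapture records captured audio input to a WAV file, apparently for the game's phone feature.
; Start and StartCapture both start the AudioCapture component and begin recording the SM_Record submix.
; Stop and StopCapture both halt capture and export the recording as "Report" to a Sound folder under the project content directory, also printing that directory.
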(event Custom|Stop
  (bind _returnvalue (Class|KismetSystemLibrary|GetProjectContentDirectory))
  (Audio|Components|Audio|Stop (Variables|Default|GetAudioCaptureComp))
  (Development|PrintString _returnvalue)
  (Class|AudioMixerBlueprintLibrary|StopRecordingOutput "WavFile" "Report" (Utilities|String|Append _returnvalue "/Sound") "/Game/Justin/Phone/SM_Record.SM_Record" 0))

(event Custom|Start
  (CameraShake|Start (Variables|Default|GetAudioCaptureComp))
  (Class|AudioMixerBlueprintLibrary|StartRecordingOutput 0.0 "/Game/Justin/Phone/SM_Record.SM_Record"))

(event EventStartCapture
  (CameraShake|Start (Variables|Default|GetAudioCaptureComp))
  (Class|AudioMixerBlueprintLibrary|StartRecordingOutput 0.0 "/Game/Justin/Phone/SM_Record.SM_Record"))

(event EventStopCapture
  (bind _returnvalue (Class|KismetSystemLibrary|GetProjectContentDirectory))
  (Audio|Components|Audio|Stop (Variables|Default|GetAudioCaptureComp))
  (Development|PrintString _returnvalue)
  (Class|AudioMixerBlueprintLibrary|StopRecordingOutput "WavFile" "Report" (Utilities|String|Append _returnvalue "/Sound") "/Game/Justin/Phone/SM_Record.SM_Record" 0))

(fn ConstructionScript)