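; BP_OmulBallon is an actor that follows the Ref component of an assigned BP_Spline actor and plays a sound once when that component stops moving.
; BeginPlay casts and caches the spline actor.
; Each Tick compares Ref's world location with the last stored one, moving the actor there if it changed.
; Otherwise it plays the sound at its own location, guarded by a flag so it never repeats.
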(event EventBeginPlay
  (bind _splineactor (Variables|Settings|GetSplineActor)
    (:then
      (bind _asbp_spline (Utilities|Casting|CastToBP_Spline _splineactor))
      (Variables|Default|SetAs%20BP%20Spline _asbp_spline))
    (:else)))

(event EventTick
  (params (DeltaSeconds :type Float%20%28single-precision%29))
  (bind _as_bp_spline (Variables|Default|GetAs%20BP%20Spline))
  (bind _ref (Variables|/Game/Justin/NPC/BP_Spline.BP_Spline_C|GetRef _as_bp_spline))
  (bind _returnvalue (Transformation|GetWorldLocation _ref))
  (if (Class|KismetMathLibrary|EqualExactlyVectorVector (Variables|Default|GetLastLocation) _returnvalue)
    (if (not (Variables|Default|Getbsoundplayed))
      (Audio|PlaySoundatLocation (Variables|Default|GetSound) (Transformation|GetActorLocation) "0, 0, 0" 1.0 1.0 0.0 0 0 0 0)
      (Variables|Default|Setbsoundplayed true))
    (else
      (Variables|Default|SetLastLocation _returnvalue)
      (Transformation|SetActorLocation _returnvalue false false))))

(fn ConstructionScript)